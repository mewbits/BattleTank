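; Player-controllable tank Blueprint that wires up firing and an orbiting aim camera.
; BeginPlay passes the barrel and turret components to SetBarrelReference and SetTurretReference, and the Fire input calls Fire, none of which are defined in these graphs.
; Aim axes rotate the camera on two separate components, yaw on the azimuth gimbal and pitch on the spring arm, scaled by CameraRotationRate without delta time.
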(event Collision|EventActorBeginOverlap
  (params (OtherActor :type Actor%20Object%20Reference)))

(event EventTick
  (params (DeltaSeconds :type Float%20%28single-precision%29)))

(event EventBeginPlay
  (Class|Tank|SetBarrelReference (Variables|Default|GetTankBarrel))
  (Class|Tank|SetTurretReference (Variables|Default|GetTankTurret)))

(event Input|ActionEvents|InputActionFire
  (params (Key :type Key%20Structure))
  (:Pressed
    (Class|Tank|Fire)))

(event Input|AxisEvents|InputAxisAimAzimuth
  (params (AxisValue :type Float%20%28single-precision%29))
  ;[1 1 1] Camera Input Binding
  (Transformation|AddLocalRotation (Variables|Default|GetAzimuthGibal) (Math|Rotator|MakeRotator 0.0 0.0 (* AxisValue (Variables|Default|GetCameraRotationRate))) false false))

(event Input|AxisEvents|InputAxisAimElevation
  (params (AxisValue :type Float%20%28single-precision%29))
  ;[1 1 1] Camera Input Binding
  (Transformation|AddLocalRotation (Variables|Default|GetSpringArm) (Math|Rotator|MakeRotator 0.0 (* AxisValue (Variables|Default|GetCameraRotationRate)) 0.0) false false))

(fn ConstructionScript)