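; Mortar_BP is a mortar enemy or emplacement Blueprint built from tank turret and barrel components.
; The construction script assigns the mortar dome and barrel meshes and sets Projectile_BP as the TankAiming component's projectile.
; On BeginPlay it initializes TankAiming with the barrel and turret so that component can drive aiming.
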(event EventBeginPlay
  (Class|TankAimingComponent|Initialize (Variables|Default|GetTankAiming) (Variables|Default|GetTankBarrel) (Variables|Default|GetTankTurret)))

(fn ConstructionScript
  (Variables|/Script/BattleTank.TankAimingComponent|SetProjectileBlueprint (Variables|Default|GetTankAiming) "/Game/Blueprints/Projectile/Projectile_BP.Projectile_BP_C")
  (Components|StaticMesh|SetStaticMesh (Variables|Default|GetTankTurret) "/Game/Meshes/Static/Mortar/mortar_dome.mortar_dome")
  (Components|StaticMesh|SetStaticMesh (Variables|Default|GetTankBarrel) "/Game/Meshes/Static/Mortar/mortar_barrel.mortar_barrel"))